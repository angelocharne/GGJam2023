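; BP_Objects1 is an object actor that randomly shows either a Rad or a Bone sprite when play begins.
; Its Box component responds only when it overlaps the player pawn's BoxComponent.
; On that contact, a DoOnce gate lets it call Hit on BP_Player with -1 a single time, then the actor destroys itself.
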(event `self.ReceiveBeginPlay`
  (bind _papersprite (`self.PaperSprite`))
  (switch `int` (`KismetMathLibrary.RandomIntegerInRange` 0 1)
    (:`0`
      (`PaperSpriteComponent.SetSprite` _papersprite "/Game/Sprites/rad_Sprite.rad_Sprite"))
    (:`1`
      (`PaperSpriteComponent.SetSprite` _papersprite "/Game/Sprites/Bone_Sprite.Bone_Sprite"))))

(event `self.Box.OnComponentBeginOverlap`
  (params (OverlappedComponent :type "PrimitiveComponent Object Reference") (OtherActor :type "Actor Object Reference") (OtherComp :type "PrimitiveComponent Object Reference") (OtherBodyIndex :type Integer) (bFromSweep :type Boolean) (SweepResult :type "HitResult Structure (by ref)"))
  (if (== OtherComp (`self.GetComponentByClass` (`GameplayStatics.GetPlayerPawn` 0) "/Script/Engine.BoxComponent"))
    (`/Engine/EditorBlueprintResources/StandardMacros.DoOnce` false
      (:`Completed`
        (bind _asbp_player (cast `/Game/Blueprints/BP_Player` (`GameplayStatics.GetPlayerPawn` 0)))
        (`/Game/Blueprints/BP_Player.Hit` _asbp_player -1)
        (`self.K2_DestroyActor`)))))

(fn `UserConstructionScript`)