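; BP_Stone is a 2D sprite hazard that hits the player on contact.
; On BeginPlay it sets its Paper sprite to a random entry from the StoneSprite array.
; When its Box overlaps the player pawn's BoxComponent, a DoOnce gate lets it call Hit on BP_Player with a negative value, then it destroys itself.
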(event `self.ReceiveBeginPlay`
  (`PaperSpriteComponent.SetSprite` (`self.PaperSprite`) (`|GetArrayItem` (`self.StoneSprite`) (`KismetMathLibrary.RandomIntegerInRange` 0 3))))

(event `self.Box.OnComponentBeginOverlap`
  (params (OverlappedComponent :type "PrimitiveComponent Object Reference") (OtherActor :type "Actor Object Reference") (OtherComp :type "PrimitiveComponent Object Reference") (OtherBodyIndex :type Integer) (bFromSweep :type Boolean) (SweepResult :type "HitResult Structure (by ref)"))
  (if (== OtherComp (`self.GetComponentByClass` (`GameplayStatics.GetPlayerPawn` 0) "/Script/Engine.BoxComponent"))
    (`/Engine/EditorBlueprintResources/StandardMacros.DoOnce` false
      (:`Completed`
        (bind _asbp_player (cast `/Game/Blueprints/BP_Player` (`GameplayStatics.GetPlayerPawn` 0)))
        (`/Game/Blueprints/BP_Player.Hit` _asbp_player -1)
        (`self.K2_DestroyActor`)))))

(fn `UserConstructionScript`)