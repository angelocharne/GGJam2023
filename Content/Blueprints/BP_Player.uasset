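; BP_Player is a player actor that moves automatically along its local up axis while the player steers it by pitching.
; Tick drives AutoMove, scaling frame time by AutoSpeed, and holds the SpringArm at a fixed world rotation, following only the actor's height with an offset below.
; MoveRight and MoveLeft add local pitch, each blocked near its 45-degree limit by a tolerance check.
; MoveForward is unused.
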(event `InputAxis|MoveForward`
  (params (AxisValue :type "Float (single-precision)")))

(event `AutoMove`
  (params (`Delta Location Z` :type "Float (double-precision)"))
  (`self.K2_AddActorLocalOffset` (`KismetMathLibrary.MakeVector` 0.0 0.0 (* `Delta Location Z` (`self.AutoSpeed`)))))

(event `InputAxis|MoveLeft`
  (params (AxisValue :type "Float (single-precision)"))
  (bind (_returnvalue_roll _returnvalue_pitch) (`KismetMathLibrary.BreakRotator` (`self.K2_GetActorRotation`)))
  (if (not (`KismetMathLibrary.NearlyEqual_FloatFloat` _returnvalue_pitch -45.0 1.0))
    (`self.K2_AddActorLocalRotation` (`KismetMathLibrary.MakeRotator` 0.0 AxisValue))))

(event `InputAxis|MoveRight`
  (params (AxisValue :type "Float (single-precision)"))
  (bind (_returnvalue_roll _returnvalue_pitch) (`KismetMathLibrary.BreakRotator` (`self.K2_GetActorRotation`)))
  (if (not (`KismetMathLibrary.NearlyEqual_FloatFloat` _returnvalue_pitch 45.0 1.0))
    (`self.K2_AddActorLocalRotation` (`KismetMathLibrary.MakeRotator` 0.0 AxisValue))))

(event `self.ReceiveTick`
  (params (DeltaSeconds :type "Float (single-precision)"))
  (bind (_returnvalue_x _returnvalue_y _returnvalue_z) (`KismetMathLibrary.BreakVector` (`self.K2_GetActorLocation`)))
  (`self.AutoMove` DeltaSeconds)
  (`SceneComponent.K2_SetWorldRotation` (`self.SpringArm`) (struct :`Yaw` -90.0) false false)
  (`SceneComponent.K2_SetWorldLocation` (`self.SpringArm`) (`KismetMathLibrary.MakeVector` 0.0 0.0 (+ _returnvalue_z -200.0)) false false))

(fn `UserConstructionScript`)