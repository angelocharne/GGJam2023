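; Death screen actor that shows one of seven Plain components according to the score in BP_GameState.
; All seven are hidden on BeginPlay.
; Every Tick, CheckScore casts the game state and runs a sequence of range checks, showing the component for the matching score band and hiding the others.
; Scores below the lowest band show none, and the top band has no upper limit.
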(event `self.ReceiveBeginPlay`
  (`SceneComponent.SetVisibility` (`self.Plain`) false false)
  (`SceneComponent.SetVisibility` (`self.Plain4`) false false)
  (`SceneComponent.SetVisibility` (`self.Plain5`) false false)
  (`SceneComponent.SetVisibility` (`self.Plain3`) false false)
  (`SceneComponent.SetVisibility` (`self.Plain2`) false false)
  (`SceneComponent.SetVisibility` (`self.Plain1`) false false)
  (`SceneComponent.SetVisibility` (`self.Plain6`) false false))

(event `CheckScore`
  (bind _plain (`self.Plain`))
  (bind _plain3 (`self.Plain3`))
  (bind _plain2 (`self.Plain2`))
  (bind _plain1 (`self.Plain1`))
  (bind _plain4 (`self.Plain4`))
  (bind _plain5 (`self.Plain5`))
  (bind _plain6 (`self.Plain6`))
  (bind _asbp_game_state (cast `/Game/Blueprints/Game/BP_GameState` (`GameplayStatics.GetGameState`)))
  (`|ExecutionSequence`
    (:`then_0`
      (bind _score (`/Game/Blueprints/Game/BP_GameState.Score` _asbp_game_state))
      (if (and (<= _score 50) (>= _score 10))
        (`SceneComponent.SetVisibility` _plain true false)
        (else
          (`SceneComponent.SetVisibility` _plain false false))))
    (:`then_1`
      (if (and (>= _score 51) (<= _score 150))
        (`SceneComponent.SetVisibility` _plain1 true false)
        (else
          (`SceneComponent.SetVisibility` _plain1 false false))))
    (:`then_2`
      (if (and (>= _score 151) (<= _score 250))
        (`SceneComponent.SetVisibility` _plain2 true false)
        (else
          (`SceneComponent.SetVisibility` _plain2 false false))))
    (:`then_3`
      (if (and (>= _score 251) (<= _score 350))
        (`SceneComponent.SetVisibility` _plain3 true false)
        (else
          (`SceneComponent.SetVisibility` _plain3 false false))))
    (:`then_4`
      (if (and (>= _score 351) (<= _score 450))
        (`SceneComponent.SetVisibility` _plain4 true false)
        (else
          (`SceneComponent.SetVisibility` _plain4 false false))))
    (:`then_5`
      (if (and (>= _score 451) (<= _score 550))
        (`SceneComponent.SetVisibility` _plain5 true false)
        (else
          (`SceneComponent.SetVisibility` _plain5 false false))))
    (:`then_6`
      (if (>= _score 551)
        (`SceneComponent.SetVisibility` _plain6 true false)
        (else
          (`SceneComponent.SetVisibility` _plain6 false false))))))

(event `self.ReceiveTick`
  (params (DeltaSeconds :type "Float (single-precision)"))
  (`self.CheckScore`))

(fn `UserConstructionScript`)