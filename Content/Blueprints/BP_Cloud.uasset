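; BP_Cloud is an ambient actor that endlessly drifts two cloud components toward target billboard markers.
; On BeginPlay it stores both clouds' start positions, starts the first loop, then starts the second after a short delay to stagger them.
; Each loop uses a timeline to lerp its cloud to its billboard's location and replays itself on finish, snapping the cloud back to the start.
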(event `CloudMove2`
  (bind (_direction _newtrack_0) (`Timeline|Timeline_0` :!via `PlayFromStart`)
    (:`Update`
      (`SceneComponent.K2_SetWorldLocation` (`self.Cloud1`) (`KismetMathLibrary.VLerp` (`self.FirstPos`) (`SceneComponent.K2_GetComponentLocation` (`self.Billboard1`)) _newtrack_0) false false))
    (:`Finished`
      (`self.CloudMove2`))))

(event `self.ReceiveBeginPlay`
  (set `self.First` (`SceneComponent.K2_GetComponentLocation` (`self.Cloud`)))
  (set `self.FirstPos` (`SceneComponent.K2_GetComponentLocation` (`self.Cloud1`)))
  (`self.MoveClouds`)
  (`KismetSystemLibrary.Delay` 2.0)
  (`self.CloudMove2`))

(event `MoveClouds`
  (bind (_direction _newtrack_0) (`Timeline|Timeline` :!via `PlayFromStart`)
    (:`Update`
      (`SceneComponent.K2_SetWorldLocation` (`self.Cloud`) (`KismetMathLibrary.VLerp` (`self.First`) (`SceneComponent.K2_GetComponentLocation` (`self.Billboard`)) _newtrack_0) false false))
    (:`Finished`
      (`self.MoveClouds`))))

(fn `UserConstructionScript`)