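; Centipede enemy that patrols back and forth through three points on a fixed-Y plane and hurts the player on contact.
; Two timelines lerp the FirstPos–ToNextPos–EndPos legs, with FlipFlops and SwitchDir chaining forward and reverse playback while rotating the flipbook.
; After a random start delay, it moves and loops an insect trill every second.
; Overlapping the player's box calls BP_Player Hit(-1), gated by a one-second DoOnce cooldown.
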(event `self.ReceiveBeginPlay`
  (`KismetSystemLibrary.Delay` (`KismetMathLibrary.RandomFloatInRange` 0.0 0.5))
  (`self.MoveToFirstPoint`)
  (`GameplayStatics.PlaySoundAtLocation` "/Game/Audio/Sound/38717__shimsewn__insect-trill.38717__shimsewn__insect-trill" (`SceneComponent.K2_GetComponentLocation` (`self.PaperFlipbook`)) (struct) 1.0 1.0 0.0 null null null null :!label _label)
  (`KismetSystemLibrary.RetriggerableDelay` 1.0)
  (goto _label))

(event `MoveToNextPoint`
  (bind _paperflipbook (`self.PaperFlipbook`))
  (`/Engine/EditorBlueprintResources/StandardMacros.FlipFlop`
    (:`A`
      (set `self.SwitchDir` true)
      (`SceneComponent.K2_SetWorldRotation` _paperflipbook (struct :`Pitch` 45.0 :`Yaw` 180.0) false false)
      (bind (_direction _newtrack_0) (`Timeline|Timeline_0` :!via `PlayFromStart` :!label _label_2)
        (:`Update`
          (bind (_returnvalue_x _returnvalue_y _returnvalue_z) (`KismetMathLibrary.BreakVector` (`KismetMathLibrary.VLerp` (`self.ToNextPos`) (`self.EndPos`) _newtrack_0)))
          (`self.K2_SetActorLocation` (`KismetMathLibrary.MakeVector` _returnvalue_x -45.0 _returnvalue_z)))
        (:`Finished`
          (if (`self.SwitchDir`)
            (`self.MoveToNextPoint`)
            (else
              (`self.MoveToFirstPoint`))))))
    (:`B`
      (set `self.SwitchDir` false)
      (`SceneComponent.K2_SetWorldRotation` _paperflipbook (struct :`Pitch` -145.0 :`Yaw` 540.0 :`Roll` 540.0) false false)
      (goto _label_2 :!via `ReverseFromEnd`))))

(event `MoveToFirstPoint`
  (bind _paperflipbook (`self.PaperFlipbook`))
  (`/Engine/EditorBlueprintResources/StandardMacros.FlipFlop`
    (:`A`
      (`SceneComponent.K2_SetWorldRotation` _paperflipbook (struct :`Pitch` -45.0 :`Yaw` 540.0 :`Roll` 540.0) false false)
      (set `self.SwitchDir` true)
      (bind (_direction _newtrack_0) (`Timeline|Timeline` :!via `PlayFromStart` :!label _label_3)
        (:`Update`
          (bind (_returnvalue_x _returnvalue_y _returnvalue_z) (`KismetMathLibrary.BreakVector` (`KismetMathLibrary.VLerp` (`self.FirstPos`) (`self.ToNextPos`) _newtrack_0)))
          (`self.K2_SetActorLocation` (`KismetMathLibrary.MakeVector` _returnvalue_x -45.0 _returnvalue_z)))
        (:`Finished`
          (if (`self.SwitchDir`)
            (`self.MoveToNextPoint`)
            (else
              (`self.MoveToFirstPoint`))))))
    (:`B`
      (`SceneComponent.K2_SetWorldRotation` _paperflipbook (struct :`Pitch` -225.0 :`Yaw` 540.0 :`Roll` 540.0) false false)
      (set `self.SwitchDir` false)
      (goto _label_3 :!via `ReverseFromEnd`))))

(event `self.Box.OnComponentBeginOverlap`
  (params (OverlappedComponent :type "PrimitiveComponent Object Reference") (OtherActor :type "Actor Object Reference") (OtherComp :type "PrimitiveComponent Object Reference") (OtherBodyIndex :type Integer) (bFromSweep :type Boolean) (SweepResult :type "HitResult Structure (by ref)"))
  (if (== OtherComp (`self.GetComponentByClass` (`GameplayStatics.GetPlayerPawn` 0) "/Script/Engine.BoxComponent"))
    (`/Engine/EditorBlueprintResources/StandardMacros.DoOnce` false :!label _label_4
      (:`Completed`
        (bind _asbp_player (cast `/Game/Blueprints/BP_Player` (`GameplayStatics.GetPlayerPawn` 0)))
        (`/Game/Blueprints/BP_Player.Hit` _asbp_player -1)
        (`KismetSystemLibrary.Delay` 1.0)
        (goto _label_4 :!via `Reset`)))))

(fn `UserConstructionScript`)