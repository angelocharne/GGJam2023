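; BP_Mole is a 2D enemy that patrols between two points and hurts the player on contact.
; After a random start delay, a FlipFlop alternately plays and reverses a Timeline, lerping X and Z at fixed Y and turning the flipbook each leg.
; A delay loop replays a dirt-drag sound every second.
; Overlap with the player's box calls Hit on BP_Player, gated by a one-second DoOnce cooldown.
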(event `self.ReceiveBeginPlay`
  (`KismetSystemLibrary.Delay` (`KismetMathLibrary.RandomFloatInRange` 0.0 0.3))
  (`self.MoveToFirstPoint`)
  (`GameplayStatics.PlaySoundAtLocation` "/Game/Audio/Sound/86988__cgeffex__drag_dirt.86988__cgeffex__drag_dirt" (`self.K2_GetActorLocation`) (struct) 1.0 1.0 0.0 null null null null :!label _label)
  (`KismetSystemLibrary.RetriggerableDelay` 1.0)
  (goto _label))

(event `MoveToFirstPoint`
  (bind _paperflipbook (`self.PaperFlipbook`))
  (`/Engine/EditorBlueprintResources/StandardMacros.FlipFlop`
    (:`A`
      (`SceneComponent.K2_SetWorldRotation` _paperflipbook (`self.StartRotation`) false false)
      (bind (_direction _newtrack_0) (`Timeline|Timeline` :!via `PlayFromStart` :!label _label_2)
        (:`Update`
          (bind (_returnvalue_x _returnvalue_y _returnvalue_z) (`KismetMathLibrary.BreakVector` (`KismetMathLibrary.VLerp` (`self.FirstPos`) (`self.ToNextPos`) _newtrack_0)))
          (`self.K2_SetActorLocation` (`KismetMathLibrary.MakeVector` _returnvalue_x -45.0 _returnvalue_z)))
        (:`Finished`
          (`self.MoveToFirstPoint`))))
    (:`B`
      (`SceneComponent.K2_SetWorldRotation` _paperflipbook (`self.ReverseRotation`) false false)
      (goto _label_2 :!via `ReverseFromEnd`))))

(event `self.Box.OnComponentBeginOverlap`
  (params (OverlappedComponent :type "PrimitiveComponent Object Reference") (OtherActor :type "Actor Object Reference") (OtherComp :type "PrimitiveComponent Object Reference") (OtherBodyIndex :type Integer) (bFromSweep :type Boolean) (SweepResult :type "HitResult Structure (by ref)"))
  (if (== OtherComp (`self.GetComponentByClass` (`GameplayStatics.GetPlayerPawn` 0) "/Script/Engine.BoxComponent"))
    (`/Engine/EditorBlueprintResources/StandardMacros.DoOnce` false :!label _label_3
      (:`Completed`
        (bind _asbp_player (cast `/Game/Blueprints/BP_Player` (`GameplayStatics.GetPlayerPawn` 0)))
        (`/Game/Blueprints/BP_Player.Hit` _asbp_player -1)
        (`KismetSystemLibrary.Delay` 1.0)
        (goto _label_3 :!via `Reset`)))))

(fn `UserConstructionScript`)