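; Ant enemy Blueprint with a Paper2D flipbook that hurts the player on contact.
; On BeginPlay it applies its RotationRate to the rotating movement, sets the flipbook's world rotation, then loops an insect trill at its location every second through a retriggerable delay.
; When its Box overlaps the player pawn's BoxComponent, it calls Hit(-1) on BP_Player, with a DoOnce and delay giving a one-second cooldown.
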(event `self.ReceiveBeginPlay`
  (set `RotatingMovementComponent.RotationRate` (`self.Rotation Rate`) (`self.RotatingMovement`))
  (`SceneComponent.K2_SetWorldRotation` (`self.PaperFlipbook`) (`self.AntRotation`) false false)
  (`GameplayStatics.PlaySoundAtLocation` "/Game/Audio/Sound/38717__shimsewn__insect-trill_me_highnote_.38717__shimsewn__insect-trill_me_highnote_" (`self.K2_GetActorLocation`) (struct) 1.0 1.0 0.0 null null null null :!label _label)
  (`KismetSystemLibrary.RetriggerableDelay` 1.0)
  (goto _label))

(event `self.Box.OnComponentBeginOverlap`
  (params (OverlappedComponent :type "PrimitiveComponent Object Reference") (OtherActor :type "Actor Object Reference") (OtherComp :type "PrimitiveComponent Object Reference") (OtherBodyIndex :type Integer) (bFromSweep :type Boolean) (SweepResult :type "HitResult Structure (by ref)"))
  (if (== OtherComp (`self.GetComponentByClass` (`GameplayStatics.GetPlayerPawn` 0) "/Script/Engine.BoxComponent"))
    (`/Engine/EditorBlueprintResources/StandardMacros.DoOnce` false :!label _label_2
      (:`Completed`
        (bind _asbp_player (cast `/Game/Blueprints/BP_Player` (`GameplayStatics.GetPlayerPawn` 0)))
        (`/Game/Blueprints/BP_Player.Hit` _asbp_player -1)
        (`KismetSystemLibrary.Delay` 1.0)
        (goto _label_2 :!via `Reset`)))))

(fn `UserConstructionScript`)