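; BP_Worm is a Paper2D hazard that patrols along X and hurts the player on contact.
; After a one-second delay, a FlipFlop alternately plays and reverses a Timeline that lerps X between FirstXPos and MovePoint, rotating the flipbook 180 degrees each turn.
; Timeline completion retriggers the FlipFlop to continue the patrol.
; Box overlap with the player pawn's box component calls Hit on BP_Player and prints the overlapping component's name.
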(event `self.ReceiveBeginPlay`
  (`KismetSystemLibrary.Delay` 1.0)
  (`self.MoveToFirstPoint`))

(event `MoveToFirstPoint`
  (bind _paperflipbook (`self.PaperFlipbook`))
  (`/Engine/EditorBlueprintResources/StandardMacros.FlipFlop`
    (:`A`
      (`SceneComponent.K2_SetWorldRotation` _paperflipbook (struct) false false)
      (bind (_direction _newtrack_0) (`Timeline|Timeline` :!via `PlayFromStart` :!label _label)
        (:`Update`
          (`self.K2_SetActorLocation` (`KismetMathLibrary.MakeVector` (`KismetMathLibrary.Lerp` (`self.FirstXPos`) (`self.MovePoint`) _newtrack_0) -50.0 (`self.New Location Z`))))
        (:`Finished`
          (`self.MoveToFirstPoint`))))
    (:`B`
      (`SceneComponent.K2_SetWorldRotation` _paperflipbook (struct :`Yaw` 180.0) false false)
      (goto _label :!via `ReverseFromEnd`))))

(event `self.Box.OnComponentBeginOverlap`
  (params (OverlappedComponent :type "PrimitiveComponent Object Reference") (OtherActor :type "Actor Object Reference") (OtherComp :type "PrimitiveComponent Object Reference") (OtherBodyIndex :type Integer) (bFromSweep :type Boolean) (SweepResult :type "HitResult Structure (by ref)"))
  (`KismetSystemLibrary.PrintString` (`KismetSystemLibrary.GetDisplayName` OtherComp))
  (if (== OtherComp (`self.GetComponentByClass` (`GameplayStatics.GetPlayerPawn` 0) "/Script/Engine.BoxComponent"))
    (bind _asbp_player (cast `/Game/Blueprints/BP_Player` (`GameplayStatics.GetPlayerPawn` 0)))
    (`/Game/Blueprints/BP_Player.Hit` _asbp_player -1)))

(fn `UserConstructionScript`)