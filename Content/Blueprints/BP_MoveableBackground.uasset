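; Endless-level background segment that fills itself with random content and chains the next segment below when the player passes through.
; BeginPlay picks a random sprite and one of twelve spawn combinations of enemies, stones, orbs and props at marker components.
; The trigger, for a living player, adds score, adjusts auto speed, spawns the next segment, then destroys this one after a delay.
; Side border overlaps flip the player's pitch.
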(event `SpawnUfo`
  (bind (_returnvalue_x _returnvalue_y _returnvalue_z) (`KismetMathLibrary.BreakVector` (`SceneComponent.K2_GetComponentLocation` (`self.Billboard12`))))
  (bind (_returnvalue_x_2 _returnvalue_y_2 _returnvalue_z_2) (`KismetMathLibrary.BreakVector` (`SceneComponent.K2_GetComponentLocation` (`self.Billboard11`))))
  (switch `int` (`KismetMathLibrary.RandomIntegerInRange` 0 1)
    (:`0`
      (bind _returnvalue (`|SpawnActorFromClass` "/Game/Blueprints/BP_Objects2.BP_Objects2_C" (`KismetMathLibrary.MakeTransform` (`KismetMathLibrary.MakeVector` _returnvalue_x_2 -45.0 _returnvalue_z_2)) "Undefined" "OverrideRootScale" null null))
      (`KismetSystemLibrary.Delay` 30.0)
      (`/Engine/EditorBlueprintResources/StandardMacros.IsValid` _returnvalue
        (:`Is Valid`
          (`self.K2_DestroyActor` _returnvalue))))
    (:`1`
      (bind _returnvalue_2 (`|SpawnActorFromClass` "/Game/Blueprints/BP_Objects2.BP_Objects2_C" (`KismetMathLibrary.MakeTransform` (`KismetMathLibrary.MakeVector` _returnvalue_x -45.0 _returnvalue_z)) "Undefined" "OverrideRootScale" null null))
      (`KismetSystemLibrary.Delay` 30.0)
      (`/Engine/EditorBlueprintResources/StandardMacros.IsValid` _returnvalue_2
        (:`Is Valid`
          (`self.K2_DestroyActor` _returnvalue_2))))))

(event `SpawnRad`
  (bind (_returnvalue_x _returnvalue_y _returnvalue_z) (`KismetMathLibrary.BreakVector` (`SceneComponent.K2_GetComponentLocation` (`self.Billboard10`))))
  (bind (_returnvalue_x_2 _returnvalue_y_2 _returnvalue_z_2) (`KismetMathLibrary.BreakVector` (`SceneComponent.K2_GetComponentLocation` (`self.Billboard9`))))
  (switch `int` (`KismetMathLibrary.RandomIntegerInRange` 0 1)
    (:`0`
      (bind _returnvalue (`|SpawnActorFromClass` "/Game/Blueprints/BP_Objects1.BP_Objects1_C" (`KismetMathLibrary.MakeTransform` (`KismetMathLibrary.MakeVector` _returnvalue_x_2 -45.0 _returnvalue_z_2)) "Undefined" "OverrideRootScale" null null))
      (`KismetSystemLibrary.Delay` 30.0)
      (`/Engine/EditorBlueprintResources/StandardMacros.IsValid` _returnvalue
        (:`Is Valid`
          (`self.K2_DestroyActor` _returnvalue))))
    (:`1`
      (bind _returnvalue_2 (`|SpawnActorFromClass` "/Game/Blueprints/BP_Objects1.BP_Objects1_C" (`KismetMathLibrary.MakeTransform` (`KismetMathLibrary.MakeVector` _returnvalue_x -45.0 _returnvalue_z)) "Undefined" "OverrideRootScale" null null))
      (`KismetSystemLibrary.Delay` 30.0)
      (`/Engine/EditorBlueprintResources/StandardMacros.IsValid` _returnvalue_2
        (:`Is Valid`
          (`self.K2_DestroyActor` _returnvalue_2))))))

(event `SpawnPipe`
  (bind (_returnvalue_x _returnvalue_y _returnvalue_z) (`KismetMathLibrary.BreakVector` (`SceneComponent.K2_GetComponentLocation` (`self.Billboard7`))))
  (bind (_returnvalue_x_2 _returnvalue_y_2 _returnvalue_z_2) (`KismetMathLibrary.BreakVector` (`SceneComponent.K2_GetComponentLocation` (`self.Billboard8`))))
  (switch `int` (`KismetMathLibrary.RandomIntegerInRange` 0 1)
    (:`0`
      (bind _returnvalue (`|SpawnActorFromClass` "/Game/Blueprints/BP_Objects.BP_Objects_C" (`KismetMathLibrary.MakeTransform` (`KismetMathLibrary.MakeVector` _returnvalue_x_2 -45.0 _returnvalue_z_2)) "Undefined" "OverrideRootScale" null null))
      (`KismetSystemLibrary.Delay` 30.0)
      (`/Engine/EditorBlueprintResources/StandardMacros.IsValid` _returnvalue
        (:`Is Valid`
          (`self.K2_DestroyActor` _returnvalue))))
    (:`1`
      (bind _returnvalue_2 (`|SpawnActorFromClass` "/Game/Blueprints/BP_Objects.BP_Objects_C" (`KismetMathLibrary.MakeTransform` (`KismetMathLibrary.MakeVector` _returnvalue_x -45.0 _returnvalue_z)) "Undefined" "OverrideRootScale" null null))
      (`KismetSystemLibrary.Delay` 30.0)
      (`/Engine/EditorBlueprintResources/StandardMacros.IsValid` _returnvalue_2
        (:`Is Valid`
          (`self.K2_DestroyActor` _returnvalue_2))))))

(event `SpawnMole`
  (bind (_returnvalue_x _returnvalue_y _returnvalue_z) (`KismetMathLibrary.BreakVector` (`SceneComponent.K2_GetComponentLocation` (`self.Pos10`))))
  (bind (_returnvalue_x_2 _returnvalue_y_2 _returnvalue_z_2) (`KismetMathLibrary.BreakVector` (`SceneComponent.K2_GetComponentLocation` (`self.Pos6`))))
  (switch `int` (`KismetMathLibrary.RandomIntegerInRange` 0 1)
    (:`0`
      (bind _returnvalue (`|SpawnActorFromClass` "/Game/Blueprints/Enemys/BP_Mole.BP_Mole_C" (`KismetMathLibrary.MakeTransform` (`KismetMathLibrary.MakeVector` _returnvalue_x -45.0 _returnvalue_z) (struct :`Yaw` 180.0 :`Roll` 180.0)) "Undefined" "OverrideRootScale" null (`SceneComponent.K2_GetComponentLocation` (`self.Pos10`)) (`SceneComponent.K2_GetComponentLocation` (`self.Pos9`)) (struct :`Yaw` 180.0 :`Roll` 180.0) (struct) null))
      (`/Engine/EditorBlueprintResources/StandardMacros.IsValid` _returnvalue
        (:`Is Valid`
          (`KismetSystemLibrary.Delay` 30.0)
          (`self.K2_DestroyActor` _returnvalue))))
    (:`1`
      (bind _returnvalue_2 (`|SpawnActorFromClass` "/Game/Blueprints/Enemys/BP_Mole.BP_Mole_C" (`KismetMathLibrary.MakeTransform` (`KismetMathLibrary.MakeVector` _returnvalue_x_2 -45.0 _returnvalue_z_2)) "Undefined" "OverrideRootScale" null (`SceneComponent.K2_GetComponentLocation` (`self.Pos6`)) (`SceneComponent.K2_GetComponentLocation` (`self.Pos7`)) (struct) (struct :`Yaw` 180.0 :`Roll` 180.0) null))
      (`/Engine/EditorBlueprintResources/StandardMacros.IsValid` _returnvalue_2
        (:`Is Valid`
          (`KismetSystemLibrary.Delay` 30.0)
          (`self.K2_DestroyActor` _returnvalue_2))))))

(event `SpawnAnt`
  (bind (_returnvalue_x _returnvalue_y _returnvalue_z) (`KismetMathLibrary.BreakVector` (`SceneComponent.K2_GetComponentLocation` (`self.Pos5`))))
  (bind (_returnvalue_x_2 _returnvalue_y_2 _returnvalue_z_2) (`KismetMathLibrary.BreakVector` (`SceneComponent.K2_GetComponentLocation` (`self.Pos5`))))
  (switch `int` (`KismetMathLibrary.RandomIntegerInRange` 0 1)
    (:`0`
      (bind _returnvalue (`|SpawnActorFromClass` "/Game/Blueprints/Enemys/BP_Ant.BP_Ant_C" (`KismetMathLibrary.MakeTransform` (`KismetMathLibrary.MakeVector` _returnvalue_x_2 -45.0 _returnvalue_z_2)) "Undefined" "OverrideRootScale" null (struct :`Pitch` -50.0) (struct :`Pitch` 180.0) null))
      (`/Engine/EditorBlueprintResources/StandardMacros.IsValid` _returnvalue
        (:`Is Valid`
          (`KismetSystemLibrary.Delay` 15.0)
          (`self.K2_DestroyActor` _returnvalue))))
    (:`1`
      (bind _returnvalue_2 (`|SpawnActorFromClass` "/Game/Blueprints/Enemys/BP_Ant.BP_Ant_C" (`KismetMathLibrary.MakeTransform` (`KismetMathLibrary.MakeVector` _returnvalue_x -45.0 _returnvalue_z)) "Undefined" "OverrideRootScale" null (struct :`Pitch` 50.0) (struct) null))
      (`/Engine/EditorBlueprintResources/StandardMacros.IsValid` _returnvalue_2
        (:`Is Valid`
          (`KismetSystemLibrary.Delay` 15.0)
          (`self.K2_DestroyActor` _returnvalue_2))))))

(event `SpawnOrbs`
  (bind (_returnvalue_x _returnvalue_y _returnvalue_z) (`KismetMathLibrary.BreakVector` (`SceneComponent.K2_GetComponentLocation` (`|GetArrayItem` (`self.OrbsPos`) (`KismetMathLibrary.RandomIntegerInRange` 0 6)))))
  (switch `int` (`KismetMathLibrary.RandomIntegerInRange` 0 3)
    (:`0`
      (set `self.Item Typ` "NewEnumerator0"))
    (:`1`
      (set `self.Item Typ` "NewEnumerator1"))
    (:`2`
      (set `self.Item Typ` "NewEnumerator2"))
    (:`3`
      (set `self.Item Typ` "NewEnumerator3")))
  (`|SpawnActorFromClass` "/Game/Blueprints/BP_Collectables.BP_Collectables_C" (`KismetMathLibrary.MakeTransform` (`KismetMathLibrary.MakeVector` _returnvalue_x -45.0 _returnvalue_z)) "Undefined" "OverrideRootScale" null (`self.Item Typ`) null))

(event `SpawnCentipede`
  (bind (_returnvalue_x _returnvalue_y _returnvalue_z) (`KismetMathLibrary.BreakVector` (`SceneComponent.K2_GetComponentLocation` (`self.Pos5`))))
  (bind (_returnvalue_x_2 _returnvalue_y_2 _returnvalue_z_2) (`KismetMathLibrary.BreakVector` (`SceneComponent.K2_GetComponentLocation` (`self.Pos4`))))
  (bind (_returnvalue_x_3 _returnvalue_y_3 _returnvalue_z_3) (`KismetMathLibrary.BreakVector` (`SceneComponent.K2_GetComponentLocation` (`self.Pos3`))))
  (bind _returnvalue (`|SpawnActorFromClass` "/Game/Blueprints/Enemys/BP_Centipede.BP_Centipede_C" (`KismetMathLibrary.MakeTransform` (`KismetMathLibrary.MakeVector` 0.0 -45.0 _returnvalue_z_3) (struct :`Pitch` 45.0)) "Undefined" "OverrideRootScale" null (`KismetMathLibrary.MakeVector` _returnvalue_x_3 0.0 _returnvalue_z_3) (`KismetMathLibrary.MakeVector` _returnvalue_x 0.0 _returnvalue_z) (`KismetMathLibrary.MakeVector` _returnvalue_x_2 0.0 _returnvalue_z_2) null))
  (set `self.Centipede` _returnvalue))

(event `SpawnEnemys`
  (bind (_returnvalue_x _returnvalue_y _returnvalue_z) (`KismetMathLibrary.BreakVector` (`SceneComponent.K2_GetComponentLocation` (`self.Pos1`))))
  (bind (_returnvalue_x_2 _returnvalue_y_2 _returnvalue_z_2) (`KismetMathLibrary.BreakVector` (`SceneComponent.K2_GetComponentLocation` (`self.Pos4`))))
  (bind (_returnvalue_x_3 _returnvalue_y_3 _returnvalue_z_3) (`KismetMathLibrary.BreakVector` (`SceneComponent.K2_GetComponentLocation` (`self.Pos3`))))
  (bind (_returnvalue_x_4 _returnvalue_y_4 _returnvalue_z_4) (`KismetMathLibrary.BreakVector` (`SceneComponent.K2_GetComponentLocation` (`self.Pos2`))))
  (bind (_returnvalue_x_5 _returnvalue_y_5 _returnvalue_z_5) (`KismetMathLibrary.BreakVector` (`SceneComponent.K2_GetComponentLocation` (`self.Pos5`))))
  (bind _returnvalue (`|SpawnActorFromClass` "/Game/Blueprints/Enemys/BP_Centipede.BP_Centipede_C" (`KismetMathLibrary.MakeTransform` (`KismetMathLibrary.MakeVector` 0.0 -45.0 _returnvalue_z_3) (struct :`Pitch` 45.0)) "Undefined" "OverrideRootScale" null (`KismetMathLibrary.MakeVector` _returnvalue_x_3 0.0 _returnvalue_z_3) (`KismetMathLibrary.MakeVector` _returnvalue_x_5 0.0 _returnvalue_z_5) (`KismetMathLibrary.MakeVector` _returnvalue_x_2 0.0 _returnvalue_z_2) null))
  (set `self.Centipede` _returnvalue)
  (bind _returnvalue_2 (`|SpawnActorFromClass` "/Game/Blueprints/Enemys/BP_Worm.BP_Worm_C" (`KismetMathLibrary.MakeTransform` (`KismetMathLibrary.MakeVector` 0.0 -45.0 _returnvalue_z) (struct :`Pitch` 45.0)) "Undefined" "OverrideRootScale" null _returnvalue_x_4 _returnvalue_z_4 _returnvalue_x (struct) (struct :`Yaw` 180.0) null))
  (set `self.Worm` _returnvalue_2))

(event `SpawnStones`
  (bind (_returnvalue_x _returnvalue_y _returnvalue_z) (`KismetMathLibrary.BreakVector` (`SceneComponent.K2_GetComponentLocation` (`|GetArrayItem` (`self.StonePos`) (`KismetMathLibrary.RandomIntegerInRange` 0 3)))))
  (bind _returnvalue (`|SpawnActorFromClass` "/Game/Blueprints/BP_Stone.BP_Stone_C" (`KismetMathLibrary.MakeTransform` (`KismetMathLibrary.MakeVector` _returnvalue_x -45.0 _returnvalue_z)) "Undefined" "OverrideRootScale" null null))
  (`KismetSystemLibrary.Delay` 30.0)
  (`/Engine/EditorBlueprintResources/StandardMacros.IsValid` _returnvalue
    (:`Is Valid`
      (`self.K2_DestroyActor` _returnvalue))))

(event `SpawnWorm`
  (bind _returnvalue_x (`KismetMathLibrary.BreakVector` (`SceneComponent.K2_GetComponentLocation` (`self.Pos2`))))
  (bind (_returnvalue_x_2 _returnvalue_y _returnvalue_z) (`KismetMathLibrary.BreakVector` (`SceneComponent.K2_GetComponentLocation` (`self.Pos1`))))
  (bind (_returnvalue_x_3 _returnvalue_y_2 _returnvalue_z_2) (`KismetMathLibrary.BreakVector` (`SceneComponent.K2_GetComponentLocation` (`self.Pos2`))))
  (bind _returnvalue_x_4 (`KismetMathLibrary.BreakVector` (`SceneComponent.K2_GetComponentLocation` (`self.Pos1`))))
  (switch `int` (`KismetMathLibrary.RandomIntegerInRange` 0 1)
    (:`0`
      (bind _returnvalue (`|SpawnActorFromClass` "/Game/Blueprints/Enemys/BP_Worm.BP_Worm_C" (`KismetMathLibrary.MakeTransform` (`KismetMathLibrary.MakeVector` _returnvalue_x_3 -45.0 _returnvalue_z_2) (struct :`Pitch` 45.0)) "Undefined" "OverrideRootScale" null _returnvalue_x_4 _returnvalue_z_2 _returnvalue_x_3 (struct :`Yaw` 180.0) (struct) null))
      (`/Engine/EditorBlueprintResources/StandardMacros.IsValid` _returnvalue
        (:`Is Valid`
          (`KismetSystemLibrary.Delay` 15.0)
          (`self.K2_DestroyActor` _returnvalue))))
    (:`1`
      (bind _returnvalue_2 (`|SpawnActorFromClass` "/Game/Blueprints/Enemys/BP_Worm.BP_Worm_C" (`KismetMathLibrary.MakeTransform` (`KismetMathLibrary.MakeVector` 0.0 -45.0 _returnvalue_z) (struct :`Pitch` 45.0)) "Undefined" "OverrideRootScale" null _returnvalue_x _returnvalue_z _returnvalue_x_2 (struct) (struct :`Yaw` 180.0) null))
      (set `self.Worm` _returnvalue_2))))

(event `self.ReceiveBeginPlay`
  (bind _orbspos (`self.OrbsPos`))
  (bind _stonepos (`self.StonePos`))
  (`PaperSpriteComponent.SetSprite` (`self.PaperSprite`) (`|GetArrayItem` (`self.New Sprite`) (`KismetMathLibrary.RandomIntegerInRange` 2 5)))
  (`KismetArrayLibrary.Array_AddUnique` _stonepos (`self.StonePos8`))
  (`KismetArrayLibrary.Array_AddUnique` _stonepos (`self.StonePos7`))
  (`KismetArrayLibrary.Array_AddUnique` _stonepos (`self.StonePos6`))
  (`KismetArrayLibrary.Array_AddUnique` _stonepos (`self.StonePos9`))
  (`KismetArrayLibrary.Array_AddUnique` _stonepos (`self.StonePos13`))
  (`KismetArrayLibrary.Array_AddUnique` _stonepos (`self.StonePos12`))
  (`KismetArrayLibrary.Array_AddUnique` _stonepos (`self.StonePos11`))
  (`KismetArrayLibrary.Array_AddUnique` _stonepos (`self.StonePos10`))
  (`KismetArrayLibrary.Array_AddUnique` _stonepos (`self.StonePos14`))
  (`KismetArrayLibrary.Array_AddUnique` _orbspos (`self.Billboard`))
  (`KismetArrayLibrary.Array_AddUnique` _orbspos (`self.Billboard6`))
  (`KismetArrayLibrary.Array_AddUnique` _orbspos (`self.Billboard5`))
  (`KismetArrayLibrary.Array_AddUnique` _orbspos (`self.Billboard2`))
  (`KismetArrayLibrary.Array_AddUnique` _orbspos (`self.Billboard4`))
  (`KismetArrayLibrary.Array_AddUnique` _orbspos (`self.Billboard3`))
  (`KismetArrayLibrary.Array_AddUnique` _orbspos (`self.Billboard1`))
  (switch `int` (`KismetMathLibrary.RandomIntegerInRange` 0 11)
    (:`0`
      (`self.SpawnStones`)
      (`self.SpawnOrbs`)
      (`self.SpawnCentipede`))
    (:`1`
      (`self.SpawnStones`)
      (`self.SpawnWorm`))
    (:`2`
      (`self.SpawnEnemys`)
      (`self.SpawnStones`))
    (:`3`
      (`self.SpawnOrbs`)
      (`self.SpawnPipe`)
      (`self.SpawnUfo`))
    (:`4`
      (`self.SpawnAnt`)
      (`self.SpawnOrbs`)
      (`self.SpawnOrbs`))
    (:`5`
      (`self.SpawnAnt`)
      (`self.SpawnEnemys`))
    (:`6`
      (`self.SpawnAnt`)
      (`self.SpawnOrbs`)
      (`self.SpawnCentipede`))
    (:`7`
      (`self.SpawnMole`)
      (`self.SpawnOrbs`)
      (`self.SpawnPipe`))
    (:`8`
      (`self.SpawnMole`)
      (`self.SpawnWorm`)
      (`self.SpawnRad`))
    (:`9`
      (`self.SpawnRad`)
      (`self.SpawnPipe`))
    (:`10`
      (`self.SpawnUfo`)
      (`self.SpawnOrbs`)
      (`self.SpawnRad`)
      (`self.SpawnAnt`))
    (:`11`
      (`self.SpawnAnt`)
      (`self.SpawnMole`)
      (`self.SpawnCentipede`)
      (`self.SpawnOrbs`))))

(event `self.PlayerTriggerBox.OnComponentBeginOverlap`
  (params (OverlappedComponent :type "PrimitiveComponent Object Reference") (OtherActor :type "Actor Object Reference") (OtherComp :type "PrimitiveComponent Object Reference") (OtherBodyIndex :type Integer) (bFromSweep :type Boolean) (SweepResult :type "HitResult Structure (by ref)"))
  (bind (_returnvalue_x _returnvalue_y _returnvalue_z) (`KismetMathLibrary.BreakVector` (`self.K2_GetActorLocation`)))
  (bind _centipede (`self.Centipede`))
  (bind _worm (`self.Worm`))
  (if (== OtherActor (`GameplayStatics.GetPlayerPawn` 0))
    (`/Engine/EditorBlueprintResources/StandardMacros.DoOnce` false
      (:`Completed`
        (bind _asbp_player (cast `/Game/Blueprints/BP_Player` (`GameplayStatics.GetPlayerPawn` 0)))
        (if (not (<= (`/Game/Blueprints/BP_Player.Health` _asbp_player) 0))
          (bind _asbp_game_state (cast `/Game/Blueprints/Game/BP_GameState` (`GameplayStatics.GetGameState`)))
          (`/Game/Blueprints/Game/BP_GameState.Add Score` _asbp_game_state 20)
          (`/Game/Blueprints/BP_Player.AddAutoSpeed` _asbp_player -20.0)
          (bind _returnvalue (`|SpawnActorFromClass` "BP_MoveableBackground_C" (`KismetMathLibrary.MakeTransform` (`KismetMathLibrary.MakeVector` 0.0 -50.0 (+ _returnvalue_z -1510.0)) (struct) (0.7 0.7 0.7)) "Undefined" "OverrideRootScale" null null))
          (`PaperSpriteComponent.SetSprite` (`/Game/Blueprints/BP_MoveableBackground.PaperSprite` _returnvalue) (`|GetArrayItem` (`self.New Sprite`) (`KismetMathLibrary.RandomIntegerInRange` 2 5)))
          (`KismetSystemLibrary.Delay` 31.0)
          (`|ExecutionSequence`
            (:`then_0`
              (`/Engine/EditorBlueprintResources/StandardMacros.IsValid` _centipede
                (:`Is Valid`
                  (`self.K2_DestroyActor` _centipede))
                (:`Is Not Valid`
                  _)))
            (:`then_1`
              (`/Engine/EditorBlueprintResources/StandardMacros.IsValid` _worm
                (:`Is Valid`
                  (`self.K2_DestroyActor` _worm))
                (:`Is Not Valid`
                  _))))
          (`self.K2_DestroyActor`))))))

(event `self.BorderRight.OnComponentBeginOverlap`
  (params (OverlappedComponent :type "PrimitiveComponent Object Reference") (OtherActor :type "Actor Object Reference") (OtherComp :type "PrimitiveComponent Object Reference") (OtherBodyIndex :type Integer) (bFromSweep :type Boolean) (SweepResult :type "HitResult Structure (by ref)"))
  (if (== OtherComp (`self.GetComponentByClass` (`GameplayStatics.GetPlayerPawn` 0) "/Script/Engine.BoxComponent"))
    (`/Engine/EditorBlueprintResources/StandardMacros.DoOnce` false :!label _label
      (:`Completed`
        (`self.K2_SetActorRotation` (`GameplayStatics.GetPlayerPawn` 0) (`KismetMathLibrary.MakeRotator` 0.0 -45.0) false)
        (goto _label :!via `Reset`)))))

(event `self.BorderLeft_0.OnComponentBeginOverlap`
  (params (OverlappedComponent :type "PrimitiveComponent Object Reference") (OtherActor :type "Actor Object Reference") (OtherComp :type "PrimitiveComponent Object Reference") (OtherBodyIndex :type Integer) (bFromSweep :type Boolean) (SweepResult :type "HitResult Structure (by ref)"))
  (`KismetSystemLibrary.PrintString` (`KismetSystemLibrary.GetDisplayName` OtherComp))
  (if (== OtherComp (`self.GetComponentByClass` (`GameplayStatics.GetPlayerPawn` 0) "/Script/Engine.BoxComponent"))
    (`/Engine/EditorBlueprintResources/StandardMacros.DoOnce` false :!label _label_2
      (:`Completed`
        (`self.K2_SetActorRotation` (`GameplayStatics.GetPlayerPawn` 0) (`KismetMathLibrary.MakeRotator` 0.0 45.0) false)
        (goto _label_2 :!via `Reset`)))))

(fn `UserConstructionScript`)