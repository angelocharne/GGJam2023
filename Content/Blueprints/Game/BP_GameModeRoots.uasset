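; Game mode that handles player death and the game-over sequence.
; Each Tick polls Died, which, once Health and ShieldPoint are depleted, stops and hides BP_Player, then possesses a BP_DeathScreen actor once.
; Its result feeds DestroyPlayer, whose DoOnce shows the MainHud game-over widget with UI-only input, then casts the current pawn to BP_Player to fade its sound and teleport it.
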(event `DestroyPlayer`
  (params (Condition :type Boolean))
  (bind _returnvalue (`GameplayStatics.GetPlayerController` 0))
  (if Condition
    (`/Engine/EditorBlueprintResources/StandardMacros.DoOnce` false
      (:`Completed`
        (bind _asmain_hud (cast `/Game/Blueprints/Game/MainHud` (`PlayerController.GetHUD` (`GameplayStatics.GetPlayerController` 0))))
        (`UserWidget.AddToViewport` (`/Game/Blueprints/Game/MainHud.GameOver` _asmain_hud) 0)
        (set `PlayerController.bShowMouseCursor` true _returnvalue)
        (`WidgetBlueprintLibrary.SetInputMode_UIOnlyEx` _returnvalue null)
        (bind _asbp_player (cast `/Game/Blueprints/BP_Player` (`GameplayStatics.GetPlayerPawn` 0)))
        (`AudioComponent.FadeOut` (`/Game/Blueprints/BP_Player.Sound` _asbp_player) 1.0 0.0 "Linear")
        (`self.K2_SetActorLocation` _asbp_player (0.0 -100.0 1000.0) false true)))))

(event `self.ReceiveTick`
  (params (DeltaSeconds :type "Float (single-precision)"))
  (bind _returnvalue (`self.Died?`))
  (`self.DestroyPlayer` _returnvalue))

(fn `Died?`
  (returns (ReturnValue :type Boolean))
  (bind _asbp_player (cast `/Game/Blueprints/BP_Player` (`GameplayStatics.GetPlayerPawn` 0)))
  (bind _returnvalue (<= (`/Game/Blueprints/BP_Player.Health` _asbp_player) 0))
  (if (and _returnvalue (<= (`/Game/Blueprints/BP_Player.ShieldPoint` _asbp_player) 0))
    (set `/Game/Blueprints/BP_Player.StopMovement` true _asbp_player)
    (set `/Game/Blueprints/BP_Player.CollectShield?` false _asbp_player)
    (`SceneComponent.SetVisibility` (`PaperCharacter.Sprite` _asbp_player) false false)
    (`/Engine/EditorBlueprintResources/StandardMacros.DoOnce` false
      (:`Completed`
        (bind _outactors (`GameplayStatics.GetAllActorsOfClass` "/Game/Blueprints/BP_DeathScreen.BP_DeathScreen_C"))
        (`Controller.Possess` (`GameplayStatics.GetPlayerController` 0) (`|GetArrayItem` _outactors))
        (return _returnvalue)))))

(fn `UserConstructionScript`)