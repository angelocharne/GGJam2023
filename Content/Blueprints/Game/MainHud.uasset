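; Main HUD that creates and holds the game's game-over, start, in-game and main menu widgets.
; On BeginPlay it adds the start screen and main menu hidden and the in-game UI visible, while the game-over screen is created but not added to the viewport.
; Helper functions set each added widget's visibility.
; EnableUiInput switches between UI-only and game-only input, toggling the mouse cursor and in-game UI to match.
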(event `self.ReceiveBeginPlay`
  (`|ExecutionSequence`
    (:`then_0`
      (bind _returnvalue (`|CreateWidget` "/Game/Blueprints/UI/WBP_GameOverScreen.WBP_GameOverScreen_C"))
      (set `self.GameOver` _returnvalue))
    (:`then_1`
      (bind _returnvalue_2 (`|CreateWidget` "/Game/Blueprints/UI/WBP_StartScreen.WBP_StartScreen_C"))
      (bind _output_get (set `self.PlayScreen` _returnvalue_2))
      (`Widget.SetVisibility` _output_get "Hidden")
      (`UserWidget.AddToViewport` _output_get 0))
    (:`then_2`
      (bind _returnvalue_3 (`|CreateWidget` "/Game/Blueprints/UI/WBP_Ingame.WBP_Ingame_C"))
      (bind _output_get_2 (set `self.UserInterFace` _returnvalue_3))
      (`Widget.SetVisibility` _output_get_2 "Visible")
      (`UserWidget.AddToViewport` _output_get_2 0))
    (:`then_3`
      (bind _returnvalue_4 (`|CreateWidget` "/Game/Blueprints/UI/WBP_MainMenu.WBP_MainMenu_C"))
      (bind _output_get_3 (set `self.MainMenu` _returnvalue_4))
      (`Widget.SetVisibility` _output_get_3 "Hidden")
      (`UserWidget.AddToViewport` _output_get_3 0))))

(fn `Enable Ui Input`
  (params (`Enable?` :type Boolean))
  (bind _returnvalue (`GameplayStatics.GetPlayerController` 0))
  (if `Enable?`
    (set `PlayerController.bShowMouseCursor` true _returnvalue)
    (`WidgetBlueprintLibrary.SetInputMode_UIOnlyEx` _returnvalue null)
    (`self.ShowUserInterFace` "Hidden")
    (else
      (set `PlayerController.bShowMouseCursor` false _returnvalue)
      (`WidgetBlueprintLibrary.SetInputMode_GameOnly` _returnvalue)
      (`self.ShowUserInterFace` "Visible"))))

(fn `ShowMainMenu`
  (params (InVisibility :type "ESlateVisibility Enum" :default "Visible"))
  (`Widget.SetVisibility` (`self.MainMenu`) InVisibility))

(fn `ShowStartScreen`
  (params (InVisibility :type "ESlateVisibility Enum" :default "Hidden"))
  (`Widget.SetVisibility` (`self.PlayScreen`) InVisibility))

(fn `ShowUserInterFace`
  (params (InVisibility :type "ESlateVisibility Enum" :default "Visible"))
  (`Widget.SetVisibility` (`self.UserInterFace`) InVisibility))

(fn `UserConstructionScript`)