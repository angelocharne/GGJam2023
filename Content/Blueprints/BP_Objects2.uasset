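; BP_Objects2 is a Paper2D UFO object that the player can collide with.
; On BeginPlay it randomly picks one of two UFO flipbooks: Ufo_Kebsmensch or Ufo_ohne_krebs_Flipbook.
; When its Box overlaps the player pawn's BoxComponent, it calls Hit on BP_Player with a negative value, then destroys itself, guarded by a DoOnce.
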(event `self.ReceiveBeginPlay`
  (bind _ufo_ohne_krebs_flipbook (`self.Ufo_ohne_krebs_Flipbook`))
  (switch `int` (`KismetMathLibrary.RandomIntegerInRange` 0 1)
    (:`0`
      (`PaperFlipbookComponent.SetFlipbook` _ufo_ohne_krebs_flipbook "/Game/Sprites/Ufo/Ufo_Kebsmensch.Ufo_Kebsmensch"))
    (:`1`
      (`PaperFlipbookComponent.SetFlipbook` _ufo_ohne_krebs_flipbook "/Game/Sprites/Ufo/Ufo_ohne_krebs_Flipbook.Ufo_ohne_krebs_Flipbook"))))

(event `self.Box.OnComponentBeginOverlap`
  (params (OverlappedComponent :type "PrimitiveComponent Object Reference") (OtherActor :type "Actor Object Reference") (OtherComp :type "PrimitiveComponent Object Reference") (OtherBodyIndex :type Integer) (bFromSweep :type Boolean) (SweepResult :type "HitResult Structure (by ref)"))
  (if (== OtherComp (`self.GetComponentByClass` (`GameplayStatics.GetPlayerPawn` 0) "/Script/Engine.BoxComponent"))
    (`/Engine/EditorBlueprintResources/StandardMacros.DoOnce` false
      (:`Completed`
        (bind _asbp_player (cast `/Game/Blueprints/BP_Player` (`GameplayStatics.GetPlayerPawn` 0)))
        (`/Game/Blueprints/BP_Player.Hit` _asbp_player -1)
        (`self.K2_DestroyActor`)))))

(fn `UserConstructionScript`)