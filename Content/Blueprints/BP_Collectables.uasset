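; Collectable pickup that appears as a sun, poop or water orb, or a shield power-up.
; On spawn, its item type selects the flipbook, and it destroys itself after a fixed lifetime.
; When its sphere overlaps the player's box component, it fires once, plays a sound and destroys itself.
; Orbs add type-specific score through BP_GameState, while the shield sets the flag and shield health on BP_Player.
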(event `self.ReceiveBeginPlay`
  (`KismetSystemLibrary.Delay` 0.01)
  (bind _asbp_game_state (cast `/Game/Blueprints/Game/BP_GameState` (`GameplayStatics.GetGameState`)))
  (set `self.GameStateREF` _asbp_game_state)
  (switch `/Game/Blueprints/E_Items` (`self.ItemTyp`)
    (:`NewEnumerator0`
      (set `self.Orb` "/Game/Sprites/SunOrb/SunOrb.SunOrb"))
    (:`NewEnumerator1`
      (set `self.Orb` "/Game/Sprites/KackiOrb/KackiOrb.KackiOrb"))
    (:`NewEnumerator2`
      (set `self.Orb` "/Game/Sprites/WaterOrb/tropfen2-Sheet1.tropfen2-Sheet1"))
    (:`NewEnumerator3`
      (set `self.Orb` "/Game/Sprites/Shield/ShieldPow.ShieldPow")))
  (`PaperFlipbookComponent.SetFlipbook` (`self.PaperFlipbook`) (`self.Orb`))
  (`KismetSystemLibrary.Delay` 30.0)
  (`self.K2_DestroyActor`))

(event `self.Sphere.OnComponentBeginOverlap`
  (params (OverlappedComponent :type "PrimitiveComponent Object Reference") (OtherActor :type "Actor Object Reference") (OtherComp :type "PrimitiveComponent Object Reference") (OtherBodyIndex :type Integer) (bFromSweep :type Boolean) (SweepResult :type "HitResult Structure (by ref)"))
  (if (== OtherComp (`self.GetComponentByClass` (`GameplayStatics.GetPlayerPawn` 0) "/Script/Engine.BoxComponent"))
    (`/Engine/EditorBlueprintResources/StandardMacros.DoOnce` false
      (:`Completed`
        (switch `/Game/Blueprints/E_Items` (`self.ItemTyp`)
          (:`NewEnumerator0`
            (set `self.How Much Score?` 20)
            (`/Game/Blueprints/Game/BP_GameState.Add Score` (`self.GameStateREF`) (`self.How Much Score?`) :!label _label)
            (`GameplayStatics.PlaySound2D` "/Game/Audio/Sound/SFX_Collect_Bright.SFX_Collect_Bright" 1.0 1.0 0.0 null null))
          (:`NewEnumerator1`
            (set `self.How Much Score?` 50)
            (goto _label))
          (:`NewEnumerator2`
            (set `self.How Much Score?` 10)
            (goto _label))
          (:`NewEnumerator3`
            (bind _asbp_player (cast `/Game/Blueprints/BP_Player` (`GameplayStatics.GetPlayerPawn` 0)))
            (set `/Game/Blueprints/BP_Player.CollectShield?` true _asbp_player)
            (`/Game/Blueprints/BP_Player.ShieldHealth` _asbp_player 1)
            (`GameplayStatics.PlaySound2D` "/Game/Audio/Sound/SFX_Collect_Gem_3.SFX_Collect_Gem_3" 1.0 1.0 0.0 null null)))
        (`self.K2_DestroyActor`)))))

(fn `UserConstructionScript`)